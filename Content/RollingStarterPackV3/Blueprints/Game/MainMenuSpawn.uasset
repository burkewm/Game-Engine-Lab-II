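; Main menu spawn platform that presents a non-physical PhysicsBall preview wearing the game instance's TemporaryMaterial.
; After BeginPlay, timelines slide four door parts open and raise an elevator that carries the spawned ball, then close the doors.
; Destroying the ball replays the sound, door and spawn sequence with a new one.
; The construction script caches rest positions, orients the direction indicator by RotateIt and toggles platform collision from HasCollision.
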(event `self.ReceiveBeginPlay`
  (bind _l_elevator (`self.L_Elevator`))
  (bind _ball (`/Game/RollingStarterPackV3/Blueprints/PhysicsBallBP.Ball` (`self.BallReference`)))
  (`KismetSystemLibrary.Delay` 0.5)
  (bind _asrolling_v3game_instance (cast `/Game/RollingStarterPackV3/Blueprints/Game/GameMode/RollingV3GameInstance` (`GameplayStatics.GetGameInstance`)))
  (set `self.Rv3Ref` _asrolling_v3game_instance)
  (`|ExecutionSequence`
    (:`then_0`
      (`GameplayStatics.PlaySound2D` "/Game/RollingStarterPackV3/Audio/Cue/Blueprints_OpenSpawn_Cue.Blueprints_OpenSpawn_Cue" 0.8 1.0 0.0 null null :!label _label)
      ;[1 1 1] Open Main Platform
      (bind (_direction _alpha) (`Timeline|DoorOpen` :!via `PlayFromStart` :!label _label_2)
        (:`Update`
          (`SceneComponent.K2_SetRelativeLocation` (`self.Part1`) (`KismetMathLibrary.VLerp` (`self.L_DoorPart1`) (40.0 -40.0 27.0) _alpha) false false)
          (`SceneComponent.K2_SetRelativeLocation` (`self.Part2`) (`KismetMathLibrary.VLerp` (`self.L_DoorPart2`) (-40.0 -40.0 27.0) _alpha) false false)
          (`SceneComponent.K2_SetRelativeLocation` (`self.Part3`) (`KismetMathLibrary.VLerp` (`self.L_DoorPart3`) (40.0 40.0 27.0) _alpha) false false)
          (`SceneComponent.K2_SetRelativeLocation` (`self.Part4`) (`KismetMathLibrary.VLerp` (`self.L_DoorPart4`) (-40.0 40.0 27.0) _alpha) false false))))
    (:`then_1`
      ;[1 1 1] Spawn PhysicsBall (control collision and physics)
      (`KismetSystemLibrary.Delay` 0.2)
      (bind _asphysics_ball_bp (castclass `/Game/RollingStarterPackV3/Blueprints/PhysicsBallBP` (`self.Class`) :!label _label_3))
      (bind _returnvalue (`|SpawnActorFromClass` _asphysics_ball_bp (`SceneComponent.K2_GetComponentToWorld` (`self.SpawnLocation`)) "AlwaysSpawn" "OverrideRootScale" null null))
      (bind _output_get (set `self.BallReference` _returnvalue))
      (`PrimitiveComponent.SetMaterial` _ball 0 (`/Game/RollingStarterPackV3/Blueprints/Game/GameMode/RollingV3GameInstance.TemporaryMaterial` (`self.Rv3Ref`)))
      (`SceneComponent.K2_SetWorldRotation` _ball (`KismetMathLibrary.MakeRotator` 0.0 0.0 (`self.Rotate It`)) false false)
      (`PrimitiveComponent.SetSimulatePhysics` _ball false)
      (`PrimitiveComponent.SetCollisionEnabled` _ball "NoCollision")
      (add `self.OnDestroyed` _output_get (delegate `Test`))
      (bind (_direction_2 _flot) (`Timeline|CapsuleMovement` :!via `PlayFromStart`)
        (:`Update`
          (`SceneComponent.K2_SetRelativeLocation` (`self.Elevator`) (`KismetMathLibrary.VLerp` _l_elevator (+ _l_elevator (0.0 0.0 200.0)) _flot) false false)
          (`SceneComponent.K2_SetRelativeLocation` (`/Game/RollingStarterPackV3/Blueprints/PhysicsBallBP.Ball` (`self.BallReference`)) (`SceneComponent.K2_GetComponentLocation` (`self.SpawnLocation`)) false false))
        (:`Finished`
          (`self.Close`))))))

(event `Close`
  (goto _label_2 :!via `ReverseFromEnd`))

(event `Test` :!signature `self.OnDestroyed`
  (params (DestroyedActor :type "Actor Object Reference"))
  ;[1 1 1] Spawn PhysicsBall (control collision and physics)
  (`|ExecutionSequence`
    (:`then_0`
      (goto _label))
    (:`then_1`
      (goto _label_3))))

(fn `UserConstructionScript`
  (set `self.L_Elevator` (`SceneComponent.RelativeLocation` (`self.Elevator`)))
  (set `self.L_Spawn` (`SceneComponent.RelativeLocation` (`self.SpawnLocation`)))
  (set `self.L_DoorPart1` (`SceneComponent.RelativeLocation` (`self.Part1`)))
  (set `self.L_DoorPart2` (`SceneComponent.RelativeLocation` (`self.Part2`)))
  (set `self.L_DoorPart3` (`SceneComponent.RelativeLocation` (`self.Part3`)))
  (set `self.L_DoorPart4` (`SceneComponent.RelativeLocation` (`self.Part4`)))
  (`SceneComponent.K2_SetRelativeRotation` (`self.SpawnDirection`) (`KismetMathLibrary.MakeRotator` 0.0 0.0 (`self.Rotate It`)) false false)
  (if (`self.HasCollision`)
    (`PrimitiveComponent.SetCollisionEnabled` (`self.SpawnPointMesh`) "QueryAndPhysics")
    (`PrimitiveComponent.SetCollisionEnabled` (`self.Part4`) "QueryAndPhysics")
    (`PrimitiveComponent.SetCollisionEnabled` (`self.Part2`) "QueryAndPhysics")
    (`PrimitiveComponent.SetCollisionEnabled` (`self.Part1`) "QueryAndPhysics")
    (`PrimitiveComponent.SetCollisionEnabled` (`self.Part3`) "QueryAndPhysics")
    (`PrimitiveComponent.SetCollisionEnabled` (`self.Elevator`) "QueryAndPhysics")
    (else
      (`PrimitiveComponent.SetCollisionEnabled` (`self.Part4`) "NoCollision")
      (`PrimitiveComponent.SetCollisionEnabled` (`self.SpawnPointMesh`) "NoCollision")
      (`PrimitiveComponent.SetCollisionEnabled` (`self.Part2`) "NoCollision")
      (`PrimitiveComponent.SetCollisionEnabled` (`self.Part1`) "NoCollision")
      (`PrimitiveComponent.SetCollisionEnabled` (`self.Part3`) "NoCollision")
      (`PrimitiveComponent.SetCollisionEnabled` (`self.Elevator`) "NoCollision"))))