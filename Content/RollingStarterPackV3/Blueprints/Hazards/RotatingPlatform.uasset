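; Rotating platform hazard that swings a pivot back and forth between zero world rotation and a target rotation, playing audio on each swing.
; The construction script maps the platform type to a PlatformData entry and applies its material.
; After a start delay, a timeline scaled to that entry's duration drives the rotation lerp.
; When each swing finishes, it pauses, then a FlipFlop alternates forward and reverse playback indefinitely.
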(event `self.ReceiveBeginPlay`
  (bind (_durationbeforestart _duration _delay _rotation) (break `/Game/RollingStarterPackV3/Blueprints/Hazards/PlatformData` (`|GetArrayItem` (`self.PlatformData`) (`self.Index`))))
  ;[1 1 1] Get type value and set timer
  (`KismetSystemLibrary.Delay` _durationbeforestart)
  (`TimelineComponent.SetPlayRate` (`self.RotatingTimeline`) (/ 1.0 _duration))
  (`AudioComponent.Play` (`self.Audio`) 0.0 :!label _label)
  (`/Engine/EditorBlueprintResources/StandardMacros.FlipFlop`
    (:`A`
      (bind (_direction _alpha) (`Timeline|RotatingTimeline` :!via `PlayFromStart` :!label _label_2)
        (:`Update`
          (`SceneComponent.K2_SetWorldRotation` (`self.Pivot`) (`KismetMathLibrary.RLerp` (struct) _rotation _alpha true) false false))
        (:`Finished`
          (`KismetSystemLibrary.Delay` _delay)
          (goto _label))))
    (:`B`
      (goto _label_2 :!via `ReverseFromEnd`))))

(fn `UserConstructionScript`
  ;[1 1 1] Set Platform Type
  (switch `/Game/RollingStarterPackV3/Blueprints/Hazards/EnumPlatform` (`self.PlatformNumber`)
    (:`NewEnumerator0`
      (set `self.Index` 0))
    (:`NewEnumerator1`
      (set `self.Index` 1))
    (:`NewEnumerator2`
      (set `self.Index` 2)))
  (`PrimitiveComponent.SetMaterial` (`self.Platform`) 0 (`.Material_14_03C0CEC44543E64615D53083CE911205` (break `/Game/RollingStarterPackV3/Blueprints/Hazards/PlatformData` (`|GetArrayItem` (`self.PlatformData`) (`self.Index`))))))