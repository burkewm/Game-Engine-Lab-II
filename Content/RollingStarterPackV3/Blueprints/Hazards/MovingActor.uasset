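; MovingActor is a hazard Blueprint that moves a child actor back and forth along a spline.
; After an initial delay on BeginPlay, a timeline with its play rate set from Duration lerps spline distance and sets the child's world location without sweeping.
; On each finish, a repeat delay and a FlipFlop alternate between reversing and replaying the timeline, producing an endless ping-pong.
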(event `self.ReceiveBeginPlay`
  (bind _spline (`self.Spline`))
  ;[1 1 1] Set timeline
  (`KismetSystemLibrary.Delay` (`self.DelayBeforeStartMoving`))
  (`TimelineComponent.SetPlayRate` (`self.SplineTimeline`) (/ 1.0 (`self.Duration`)))
  ;[1 1 1] Follow spline from begining till end
  (bind (_direction _alpha) (`Timeline|SplineTimeline` :!label _label)
    (:`Update`
      (`SceneComponent.K2_SetWorldLocation` (`self.ChildActor`) (`SplineComponent.GetLocationAtDistanceAlongSpline` _spline (`KismetMathLibrary.Lerp` 0.0 (`SplineComponent.GetSplineLength` _spline) _alpha) "World") false false))
    (:`Finished`
      (`KismetSystemLibrary.Delay` (`self.DelayBeforeRepeat`))
      (`/Engine/EditorBlueprintResources/StandardMacros.FlipFlop`
        (:`A`
          (goto _label :!via `Reverse`))
        (:`B`
          (goto _label))))))

(fn `UserConstructionScript`)