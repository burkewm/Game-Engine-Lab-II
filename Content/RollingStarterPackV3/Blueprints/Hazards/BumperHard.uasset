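; Hazard bumper that knocks the PhysicsBallBP ball away on hit with an impulse, animation, pulse effect and sound.
; Construction script sets crystal material and trigger spheres per mode: Easy stays passive, Medium and Hard hide the bumper until approached.
; On inner overlap, Medium launches itself at the player's predicted position, while Hard runs AIMoveTo first.
; A second later the top detaches and bumping stops; simulated parts receive custom gravity along GravityRoot.
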(event `self.Bumpher.OnComponentHit`
  (params (HitComponent :type "PrimitiveComponent Object Reference") (OtherActor :type "Actor Object Reference") (OtherComp :type "PrimitiveComponent Object Reference") (NormalImpulse :type "Vector Structure") (Hit :type "HitResult Structure (by ref)"))
  ;[1 1 1] On event hit plays animation and add impusle to it
  (if (`self.DidntAttack`)
    (set `self.Location` (`.Location` (`GameplayStatics.BreakHitResult` Hit)))
    (bind _asphysics_ball_bp (cast `/Game/RollingStarterPackV3/Blueprints/PhysicsBallBP` OtherActor))
    (bind _ball (`/Game/RollingStarterPackV3/Blueprints/PhysicsBallBP.Ball` _asphysics_ball_bp))
    (`PrimitiveComponent.AddImpulse` _ball (* (`KismetMathLibrary.Conv_RotatorToVector` (`KismetMathLibrary.FindLookAtRotation` (`SceneComponent.K2_GetComponentLocation` (`self.Root`)) (`SceneComponent.K2_GetComponentLocation` _ball))) (`self.BumperForce`)) "None" false)
    (`|ExecutionSequence` :!label _label
      (:`then_0`
        (bind (_direction _newtrack_0) (`Timeline|BumperTimeline` :!via `PlayFromStart`)
          (:`Update`
            (`SceneComponent.K2_SetRelativeLocation` (`self.Bumpher`) (`KismetMathLibrary.VLerp` (`self.Relative Location`) (0.0 0.0 -45.0) _newtrack_0) false false)
            (`MaterialInstanceDynamic.SetScalarParameterValue` (`self.MaterialRef`) "Amount" _newtrack_0))))
      (:`then_1`
        (`GameplayStatics.SpawnEmitterAtLocation` "/Game/RollingStarterPackV3/Effects/P_Pulse_Ring2.P_Pulse_Ring2" (`self.Location`))
        (`GameplayStatics.PlaySound2D` "/Game/RollingStarterPackV3/Audio/Wav/BumperR.BumperR" 1.0 1.0 0.0 null null)))))

(event `self.BumperBase.OnComponentHit`
  (params (HitComponent :type "PrimitiveComponent Object Reference") (OtherActor :type "Actor Object Reference") (OtherComp :type "PrimitiveComponent Object Reference") (NormalImpulse :type "Vector Structure") (Hit :type "HitResult Structure (by ref)"))
  ;[1 1 1] On event hit plays animation and add impusle to it
  (if (`self.DidntAttack`)
    (set `self.Location` (`.Location` (`GameplayStatics.BreakHitResult` Hit)))
    (bind _asphysics_ball_bp (cast `/Game/RollingStarterPackV3/Blueprints/PhysicsBallBP` OtherActor))
    (bind _ball (`/Game/RollingStarterPackV3/Blueprints/PhysicsBallBP.Ball` _asphysics_ball_bp))
    (`PrimitiveComponent.AddImpulse` _ball (* (`KismetMathLibrary.Conv_RotatorToVector` (`KismetMathLibrary.FindLookAtRotation` (`SceneComponent.K2_GetComponentLocation` (`self.Root`)) (`SceneComponent.K2_GetComponentLocation` _ball))) (`self.BumperForce`)) "None" false)
    (goto _label)))

(event `self.ReceiveTick`
  (params (DeltaSeconds :type "Float (single-precision)"))
  (bind _bumperbase (`self.BumperBase`))
  (bind _bumpher (`self.Bumpher`))
  (bind _returnvalue (* (`SceneComponent.GetUpVector` (`self.GravityRoot`)) (`self.Temporary Gravity Force`)))
  ;[1 1 1] Adds Gravity
  (if (`SceneComponent.IsSimulatingPhysics` _bumperbase "None")
    (`PrimitiveComponent.AddForce` _bumperbase _returnvalue "None" true)
    (if (`SceneComponent.IsSimulatingPhysics` _bumpher "None")
      (`PrimitiveComponent.AddForce` _bumpher _returnvalue "None" true))))

(event `self.NotifyColision.OnComponentBeginOverlap`
  (params (OverlappedComponent :type "PrimitiveComponent Object Reference") (OtherActor :type "Actor Object Reference") (OtherComp :type "PrimitiveComponent Object Reference") (OtherBodyIndex :type Integer) (bFromSweep :type Boolean) (SweepResult :type "HitResult Structure (by ref)"))
  ;[1 1 1] Medium Mode Notify player
  (cast `/Game/RollingStarterPackV3/Blueprints/PhysicsBallBP` OtherActor)
  (if (not (and (`SceneComponent.IsSimulatingPhysics` (`self.BumperBase`) "None") (`|EnumInequality` (`self.Mode`) "NewEnumerator0")))
    (bind (_direction _newtrack_0) (`Timeline|Activation` :!via `PlayFromStart` :!label _label_2)
      (:`Update`
        (`SceneComponent.K2_SetRelativeLocation` (`self.Bumpher`) (`KismetMathLibrary.MakeVector` 0.0 0.0 (`KismetMathLibrary.Lerp` -75.0 0.0 _newtrack_0)) false false)))))

(event `self.NotifyColision.OnComponentEndOverlap`
  (params (OverlappedComponent :type "PrimitiveComponent Object Reference") (OtherActor :type "Actor Object Reference") (OtherComp :type "PrimitiveComponent Object Reference") (OtherBodyIndex :type Integer))
  ;[1 1 1] Medium Mode Notify player
  (cast `/Game/RollingStarterPackV3/Blueprints/PhysicsBallBP` OtherActor)
  (if (not (and (`SceneComponent.IsSimulatingPhysics` (`self.BumperBase`) "None") (`|EnumInequality` (`self.Mode`) "NewEnumerator0")))
    (goto _label_2 :!via `ReverseFromEnd`)))

(event `self.ActivationColision.OnComponentBeginOverlap`
  (params (OverlappedComponent :type "PrimitiveComponent Object Reference") (OtherActor :type "Actor Object Reference") (OtherComp :type "PrimitiveComponent Object Reference") (OtherBodyIndex :type Integer) (bFromSweep :type Boolean) (SweepResult :type "HitResult Structure (by ref)"))
  (bind _returnvalue (`GameplayStatics.GetPlayerPawn` 0))
  (bind _returnvalue_2 (`GameplayStatics.GetPlayerPawn` 0))
  (bind _bumpher (`self.Bumpher`))
  ;[1 1 1] Select base on mode
  (cast `/Game/RollingStarterPackV3/Blueprints/PhysicsBallBP` OtherActor)
  (`/Engine/EditorBlueprintResources/StandardMacros.DoOnce` false
    (:`Completed`
      (if (`|EnumEquality` (`self.Mode`) "NewEnumerator2")
        (`PrimitiveComponent.SetSimulatePhysics` (`self.BumperBase`) true)
        ;[1 1 1] Follow PLayer
        (bind _output_get (set `self.Distance` (`KismetMathLibrary.VSize` (- (`self.K2_GetActorLocation` (`GameplayStatics.GetPlayerPawn` 0)) (`SceneComponent.K2_GetComponentLocation` (`self.BumperBase`))))))
        (set `self.Time` (/ _output_get 3000.0))
        (bind _output_get_2 (set `self.PredictLocation` (+ (`self.K2_GetActorLocation` _returnvalue) (* (`self.GetVelocity` _returnvalue) (`self.Time`)))))
        (`|AIMoveTo` self _output_get_2 (`GameplayStatics.GetPlayerPawn` 0) 500.0
          (:`OnSuccess`
            _)
          (:`OnFail`
            _))
        (else
          (`PrimitiveComponent.SetSimulatePhysics` (`self.BumperBase`) true)))
      ;[1 1 1] Shoots itself into player trys to predict his movement
      (bind _output_get_3 (set `self.Distance` (`KismetMathLibrary.VSize` (- (`self.K2_GetActorLocation` (`GameplayStatics.GetPlayerPawn` 0)) (`SceneComponent.K2_GetComponentLocation` (`self.BumperBase`))))))
      (set `self.Time` (/ _output_get_3 3000.0))
      (bind _output_get_4 (set `self.PredictLocation` (+ (`self.K2_GetActorLocation` _returnvalue_2) (* (`self.GetVelocity` _returnvalue_2) (`self.Time`)))))
      (`PrimitiveComponent.AddImpulse` (`self.BumperBase`) (* (`KismetMathLibrary.Conv_RotatorToVector` (`KismetMathLibrary.FindLookAtRotation` (`SceneComponent.K2_GetComponentLocation` (`self.BumperBase`)) _output_get_4)) (`self.BumperForce`)) "None" false)
      (`KismetSystemLibrary.Delay` 1.0)
      ;[1 1 1] Disable Bumper
      (`SceneComponent.K2_DetachFromComponent` _bumpher "KeepWorld" "KeepWorld" "KeepWorld" true)
      (`PrimitiveComponent.SetSimulatePhysics` _bumpher true)
      (`PrimitiveComponent.AddImpulse` _bumpher (* (`SceneComponent.GetUpVector` (`self.GravityRoot`)) 50000.0) "None" false)
      (set `self.DidntAttack` false)
      (`MaterialInstanceDynamic.SetScalarParameterValue` (`self.MaterialRef`) "Amount" 1.0))))

(fn `UserConstructionScript`
  (locals (BumperColor :type "MaterialInterface Object Reference" :default "/Game/RollingStarterPackV3/RollingPack/Materials/M_CrystalMaterialHard_Inst.M_CrystalMaterialHard_Inst"))
  (bind _notifycolision (`self.NotifyColision`))
  (bind _notifycolision_2 (`self.NotifyColision`))
  (bind _sphereradius (`self.SphereRadius`))
  (if (not (`self.Refresh`))
    (set `self.Refresh` true)
    (set `self.Mode` "NewEnumerator0"))
  (set `self.Relative Location` (`KismetMathLibrary.MakeVector` (.x (`SceneComponent.RelativeLocation` (`self.Bumpher`))) (.y (`SceneComponent.RelativeLocation` (`self.Bumpher`))) (+ (.z (`SceneComponent.RelativeLocation` (`self.Bumpher`))) 75.0)))
  ;[1 1 1] Select mode
  (switch `/Game/RollingStarterPackV3/Blueprints/Hazards/EnumMode` (`self.Mode`)
    (:`NewEnumerator0`
      (set `local.BumperColor` "/Game/RollingStarterPackV3/Materials/M_Inst/M_CrystalMaterialEasy_Inst.M_CrystalMaterialEasy_Inst")
      (`SceneComponent.K2_SetRelativeLocation` (`self.Bumpher`) (0.0 0.0 0.0) false false)
      (`SceneComponent.SetVisibility` _notifycolision false false)
      (`SceneComponent.SetVisibility` (`self.ActivationColision`) false false)
      (set `PrimitiveComponent.bGenerateOverlapEvents` false (`self.ActivationColision`))
      (set `PrimitiveComponent.bGenerateOverlapEvents` false _notifycolision))
    (:`NewEnumerator1`
      (set `local.BumperColor` "/Game/RollingStarterPackV3/Materials/M_Inst/M_CrystalMaterialMedium_Inst.M_CrystalMaterialMedium_Inst")
      (`SceneComponent.K2_SetRelativeLocation` (`self.Bumpher`) (0.0 0.0 -75.0) false false :!label _label)
      (`SceneComponent.SetVisibility` _notifycolision_2 true false)
      (`SceneComponent.SetVisibility` (`self.ActivationColision`) true false)
      (set `PrimitiveComponent.bGenerateOverlapEvents` true _notifycolision_2)
      (set `PrimitiveComponent.bGenerateOverlapEvents` true (`self.ActivationColision`))
      (`SphereComponent.SetSphereRadius` (`self.ActivationColision`) _sphereradius true)
      (`SphereComponent.SetSphereRadius` (`self.NotifyColision`) (* _sphereradius 1.4) true))
    (:`NewEnumerator2`
      (set `local.BumperColor` "/Game/RollingStarterPackV3/Materials/M_Inst/M_CrystalMaterialHard_Inst.M_CrystalMaterialHard_Inst")
      (goto _label)))
  (bind _returnvalue (`PrimitiveComponent.CreateDynamicMaterialInstance` (`self.Bumpher`) 3 (`local.BumperColor`) "None"))
  (set `self.MaterialRef` _returnvalue)
  (`MaterialInstanceDynamic.SetScalarParameterValue` (`self.MaterialRef`) "Amount" 0.0))