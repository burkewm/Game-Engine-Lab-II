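; Ventilator hazard that blows the player's physics ball along the direction of its Arrow component while the ball is inside the impulse capsule.
; Overlap begin starts a fast looping timer that applies AirForce as an acceleration, and overlap end pauses it.
; The construction script sizes the capsule from Radius and HalfHeight and raises it so its base sits at its parent's origin.
; Tick spins the fan mesh at a frame-rate-dependent speed.
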(event `self.ReceiveTick`
  (params (DeltaSeconds :type "Float (single-precision)"))
  (`SceneComponent.K2_AddRelativeRotation` (`self.Vetilator`) (struct :`Roll` 1.0) false false))

(event `self.ImpulseField.OnComponentEndOverlap`
  (params (OverlappedComponent :type "PrimitiveComponent Object Reference") (OtherActor :type "Actor Object Reference") (OtherComp :type "PrimitiveComponent Object Reference") (OtherBodyIndex :type Integer))
  (cast `/Game/RollingStarterPackV3/Blueprints/PhysicsBallBP` OtherActor)
  (`KismetSystemLibrary.K2_PauseTimerHandle` (stale `self.ImpulseField.OnComponentBeginOverlap` _returnvalue)))

(event `self.ImpulseField.OnComponentBeginOverlap`
  (params (OverlappedComponent :type "PrimitiveComponent Object Reference") (OtherActor :type "Actor Object Reference") (OtherComp :type "PrimitiveComponent Object Reference") (OtherBodyIndex :type Integer) (bFromSweep :type Boolean) (SweepResult :type "HitResult Structure (by ref)"))
  (bind _asphysics_ball_bp (cast `/Game/RollingStarterPackV3/Blueprints/PhysicsBallBP` OtherActor))
  (bind _returnvalue (`KismetSystemLibrary.K2_SetTimerDelegate` (delegate `CustomEvent`) 0.01 true)))

(event `CustomEvent`
  (`/Engine/EditorBlueprintResources/StandardMacros.IsValid` (stale `self.ImpulseField.OnComponentBeginOverlap` _asphysics_ball_bp)
    (:`Is Valid`
      (`PrimitiveComponent.AddForce` (`/Game/RollingStarterPackV3/Blueprints/PhysicsBallBP.Ball` (stale `self.ImpulseField.OnComponentBeginOverlap` _asphysics_ball_bp)) (* (`SceneComponent.GetForwardVector` (`self.Arrow`)) (`self.AirForce`)) "None" true))))

(fn `UserConstructionScript`
  (bind _impulsefield (`self.ImpulseField`))
  (`CapsuleComponent.SetCapsuleHalfHeight` _impulsefield (`self.HalfHeight`) true)
  (`CapsuleComponent.SetCapsuleRadius` _impulsefield (`self.Radius`) true)
  (`SceneComponent.K2_SetRelativeLocation` (`self.ImpulseField`) (`KismetMathLibrary.MakeVector` 0.0 0.0 (`self.HalfHeight`)) false false))