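; Player-aimed cannon hazard for the rolling ball game that captures the ball and launches it where the camera points.
; Overlapping the trigger freezes the ball's physics, eases it into the cannon, and possesses the cannon with a camera blend.
; Mouse or gamepad aims the pitch-clamped camera.
; Jump fires an impulse along camera forward, returns possession and view to the ball with matched yaw, and briefly disables cannon collision to avoid snagging.
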(event `InputAxis|LookUp`
  (params (AxisValue :type "Float (single-precision)"))
  (bind _lookuplimit (`self.LookUpLimit`))
  (`SceneComponent.K2_SetRelativeRotation` (`self.Camera`) (`KismetMathLibrary.MakeRotator` (.roll (`SceneComponent.RelativeRotation` (`self.Camera`))) (`KismetMathLibrary.ClampAngle` (+ (.pitch (`SceneComponent.RelativeRotation` (`self.Camera`))) (* AxisValue (`self.MouseLookUpRate`))) (- 0.0 _lookuplimit) _lookuplimit) (.yaw (`SceneComponent.RelativeRotation` (`self.Camera`)))) false false))

(event `InputAxis|Turn`
  (params (AxisValue :type "Float (single-precision)"))
  (`SceneComponent.K2_AddRelativeRotation` (`self.Camera`) (`KismetMathLibrary.MakeRotator` 0.0 0.0 (* AxisValue (`self.MouseTurnRate`))) false false))

(event `InputAxis|GamepadTurn`
  (params (AxisValue :type "Float (single-precision)"))
  (`SceneComponent.K2_AddRelativeRotation` (`self.Camera`) (`KismetMathLibrary.MakeRotator` 0.0 0.0 (* AxisValue (`self.GamepadTurnRation`) (`GameplayStatics.GetWorldDeltaSeconds`))) false false))

(event `InputAxis|GamepadLookUp`
  (params (AxisValue :type "Float (single-precision)"))
  (bind _lookuplimit (`self.LookUpLimit`))
  (`SceneComponent.K2_SetRelativeRotation` (`self.Camera`) (`KismetMathLibrary.MakeRotator` (.roll (`SceneComponent.RelativeRotation` (`self.Camera`))) (`KismetMathLibrary.ClampAngle` (+ (.pitch (`SceneComponent.RelativeRotation` (`self.Camera`))) (* AxisValue (`self.GamepadLookUpRation`) (`GameplayStatics.GetWorldDeltaSeconds`))) (- 0.0 _lookuplimit) _lookuplimit) (.yaw (`SceneComponent.RelativeRotation` (`self.Camera`)))) false false))

(event `self.PossesCollision.OnComponentBeginOverlap`
  (params (OverlappedComponent :type "PrimitiveComponent Object Reference") (OtherActor :type "Actor Object Reference") (OtherComp :type "PrimitiveComponent Object Reference") (OtherBodyIndex :type Integer) (bFromSweep :type Boolean) (SweepResult :type "HitResult Structure (by ref)"))
  (bind _returnvalue (`GameplayStatics.GetPlayerController` 0))
  ;[1 1 1] Posses Cannon and blender camera
  (bind _asphysics_ball_bp (cast `/Game/RollingStarterPackV3/Blueprints/PhysicsBallBP` OtherActor))
  (set `self.BallRef` _asphysics_ball_bp)
  (`GameplayStatics.PlaySound2D` "/Game/RollingStarterPackV3/Audio/Wav/CannonIn.CannonIn" 1.0 1.0 0.0 null null)
  (`PrimitiveComponent.SetSimulatePhysics` (`/Game/RollingStarterPackV3/Blueprints/PhysicsBallBP.Ball` (`self.BallRef`)) false)
  (`|ExecutionSequence`
    (:`then_0`
      (`KismetSystemLibrary.MoveComponentTo` (`/Game/RollingStarterPackV3/Blueprints/PhysicsBallBP.Ball` (`self.BallRef`)) (`SceneComponent.K2_GetComponentLocation` (`self.Cannon`)) (struct) false true 1.0 true)
      (`Controller.Possess` _returnvalue self))
    (:`then_1`
      (`PlayerController.SetViewTargetWithBlend` _returnvalue self 1.0 "VTBlend_Linear" 0.5 false))))

(event `InputAction|Jump`
  (params (Key :type "Key Structure"))
  ;[1 1 1] Fire Cannon Disable Cannon Collision so the ball does not get stuck in it
  (:`Pressed`
    (`PrimitiveComponent.SetSimulatePhysics` (`/Game/RollingStarterPackV3/Blueprints/PhysicsBallBP.Ball` (`self.BallRef`)) true)
    (`PrimitiveComponent.SetCollisionEnabled` (`self.Cannon`) "NoCollision")
    (`PrimitiveComponent.AddImpulse` (`/Game/RollingStarterPackV3/Blueprints/PhysicsBallBP.Ball` (`self.BallRef`)) (* (`SceneComponent.GetForwardVector` (`self.Camera`)) (`self.FirePower`)) "None" false)
    (`SceneComponent.K2_SetRelativeRotation` (`/Game/RollingStarterPackV3/Blueprints/PhysicsBallBP.CameraBoom` (`self.BallRef`)) (`KismetMathLibrary.MakeRotator` (.roll (`SceneComponent.RelativeRotation` (`/Game/RollingStarterPackV3/Blueprints/PhysicsBallBP.CameraBoom` (`self.BallRef`)))) (.pitch (`SceneComponent.RelativeRotation` (`/Game/RollingStarterPackV3/Blueprints/PhysicsBallBP.CameraBoom` (`self.BallRef`)))) (.yaw (`SceneComponent.K2_GetComponentRotation` (`self.Camera`)))) false false)
    (`GameplayStatics.PlaySound2D` "/Game/RollingStarterPackV3/Audio/Cue/CannonShootNew_Cue.CannonShootNew_Cue" 1.0 1.0 0.0 null null)
    (`PlayerController.SetViewTargetWithBlend` (`GameplayStatics.GetPlayerController` 0) (`self.BallRef`) 1.0 "VTBlend_Linear" 0.2 false)
    (`Controller.Possess` (`GameplayStatics.GetPlayerController` 0) (`self.BallRef`))
    (`KismetSystemLibrary.Delay` 1.0)
    (`PrimitiveComponent.SetCollisionEnabled` (`self.Cannon`) "QueryAndPhysics")))

(fn `UserConstructionScript`)