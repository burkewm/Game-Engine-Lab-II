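; Cannon hazard that turns toward the player inside its box and fires projectiles at the PhysicsBallBP.
; After a start delay, a looping timer plays the recoil timeline and sound, then spawns shots aimed at the player's velocity-predicted position with random spread.
; Leaving the box pauses the timer, and the ball's destruction also requests a pause.
; The construction script uses Mode to set core material, projectile class, speed and fire rate.
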(event `self.ReceiveTick`
  (params (DeltaSeconds :type "Float (single-precision)"))
  (bind _returnvalue (`GameplayStatics.GetPlayerPawn` 0))
  (bind _returnvalue_2 (`KismetMathLibrary.FindLookAtRotation` (`SceneComponent.K2_GetComponentLocation` (`self.CannonHolder`)) (`self.K2_GetActorLocation` _returnvalue)))
  ;[1 1 1] Control Rotation
  (if (`PrimitiveComponent.IsOverlappingActor` (`self.Box`) _returnvalue)
    (`SceneComponent.K2_SetWorldRotation` (`self.CannonHolder`) (`KismetMathLibrary.RInterpTo` (`KismetMathLibrary.MakeRotator` (- 0.0 (.pitch _returnvalue_2)) (.roll _returnvalue_2) (+ (.yaw _returnvalue_2) -90.0)) (`SceneComponent.K2_GetComponentRotation` (`self.CannonHolder`)) (`GameplayStatics.GetWorldDeltaSeconds`) 0.01) false false)
    (set `self.EndLocation` (* (`KismetMathLibrary.GetForwardVector` _returnvalue_2) -35.0))))

(event `self.Box.OnComponentBeginOverlap`
  (params (OverlappedComponent :type "PrimitiveComponent Object Reference") (OtherActor :type "Actor Object Reference") (OtherComp :type "PrimitiveComponent Object Reference") (OtherBodyIndex :type Integer) (bFromSweep :type Boolean) (SweepResult :type "HitResult Structure (by ref)"))
  (bind _returnvalue (`GameplayStatics.GetPlayerPawn` 0))
  (bind _startlocation (`self.StartLocation`))
  (bind _returnvalue_2 (`SceneComponent.K2_GetComponentLocation` (`self.Muzzle`)))
  (bind _asphysics_ball_bp (cast `/Game/RollingStarterPackV3/Blueprints/PhysicsBallBP` OtherActor))
  (bind _output_get (set `self.BallRef` _asphysics_ball_bp))
  (add `self.OnDestroyed` _output_get (delegate `Destroyed`))
  (`KismetSystemLibrary.Delay` (`self.DelayBeforeFire`))
  (`|ExecutionSequence`
    (:`then_0`
      (bind _returnvalue_3 (`KismetSystemLibrary.K2_SetTimerDelegate` (delegate `Fire`) (/ 1.0 (`self.FireRatePerSecond`)) true)))
    (:`then_1`
      (`|ExecutionSequence`
        (:`then_0`
          ;[1 1 1] Shoot Animation
          (bind (_direction _newtrack_0) (`Timeline|FireAnimation` :!via `PlayFromStart` :!label _label)
            (:`Update`
              (`SceneComponent.K2_SetRelativeLocation` (`self.CannonHolder`) (`KismetMathLibrary.VLerp` _startlocation (+ _startlocation (`self.EndLocation`)) _newtrack_0) false false))))
        (:`then_1`
          (`GameplayStatics.PlaySoundAtLocation` "/Game/RollingStarterPackV3/Audio/Wav/CannonShoot.CannonShoot" (`SceneComponent.K2_GetComponentLocation` (`self.Muzzle`)) (struct) 0.25 1.0 0.0 "/Game/RollingStarterPackV3/Audio/LongAttenutation.LongAttenutation" null null :!label _label_2)
          ;[1 1 1] Predict Movement shot location
          (bind _output_get_2 (set `self.Distance` (`KismetMathLibrary.VSize` (- (`self.K2_GetActorLocation` (`GameplayStatics.GetPlayerPawn` 0)) (`SceneComponent.K2_GetComponentLocation` (`self.Muzzle`))))))
          (set `self.Time` (/ _output_get_2 (`self.ProjectileVelocity`)))
          (bind _output_get_3 (set `self.PredictLocation` (+ (`self.K2_GetActorLocation` _returnvalue) (* (`self.GetVelocity` _returnvalue) (`self.Time`)) (0.0 0.0 0.0))))
          (`KismetSystemLibrary.LineTraceSingle` _returnvalue_2 _output_get_3 "TraceTypeQuery1")
          (`|SpawnActorFromClass` (`self.Class`) (`KismetMathLibrary.MakeTransform` _returnvalue_2 (`KismetMathLibrary.MakeRotator` (.roll (`KismetMathLibrary.FindLookAtRotation` _returnvalue_2 (`self.PredictLocation`))) (- (.pitch (`KismetMathLibrary.FindLookAtRotation` _returnvalue_2 (`self.PredictLocation`))) (`KismetMathLibrary.RandomFloatInRange` 3.0 -3.0)) (- (.yaw (`KismetMathLibrary.FindLookAtRotation` _returnvalue_2 (`self.PredictLocation`))) (`KismetMathLibrary.RandomFloatInRange` 3.0 -3.0))) (0.5 0.5 0.5)) "Undefined" "OverrideRootScale" null null))))))

(event `Fire`
  (`TimelineComponent.SetPlayRate` (`self.FireAnimation`) (`self.FireRatePerSecond`))
  (`|ExecutionSequence`
    (:`then_0`
      (goto _label :!via `PlayFromStart`))
    (:`then_1`
      (goto _label_2))))

(event `Destroyed` :!signature `self.OnDestroyed`
  (params (DestroyedActor :type "Actor Object Reference"))
  (`KismetSystemLibrary.K2_PauseTimer` null "Fire"))

(event `self.Box.OnComponentEndOverlap`
  (params (OverlappedComponent :type "PrimitiveComponent Object Reference") (OtherActor :type "Actor Object Reference") (OtherComp :type "PrimitiveComponent Object Reference") (OtherBodyIndex :type Integer))
  (bind _asphysics_ball_bp (cast `/Game/RollingStarterPackV3/Blueprints/PhysicsBallBP` OtherActor))
  (set `self.BallRef` _asphysics_ball_bp)
  (`KismetSystemLibrary.K2_PauseTimerHandle` (stale `self.Box.OnComponentBeginOverlap` _returnvalue_3)))

(fn `UserConstructionScript`
  (bind _core (`self.Core`))
  ;[1 1 1] Set Mode
  (set `self.StartLocation` (`SceneComponent.RelativeLocation` (`self.CannonHolder`)))
  (`BoxComponent.SetBoxExtent` (`self.Box`) (`self.BoxRadius`) true)
  (switch `/Game/RollingStarterPackV3/Blueprints/Hazards/EnumMode` (`self.Mode`)
    (:`NewEnumerator0`
      (`PrimitiveComponent.SetMaterial` _core 0 "/Game/RollingStarterPackV3/Materials/M_Inst/M_LightGreen_Inst.M_LightGreen_Inst")
      (set `self.ProjectileVelocity` 3000.0)
      (set `self.FireRatePerSecond` 1.0)
      (set `self.Class` "/Game/RollingStarterPackV3/Blueprints/Hazards/Projectiles/Cannon_ProjectileEasy.Cannon_ProjectileEasy_C"))
    (:`NewEnumerator1`
      (`PrimitiveComponent.SetMaterial` _core 0 "/Game/RollingStarterPackV3/Materials/M_Inst/M_LightYellow_Inst.M_LightYellow_Inst")
      (set `self.ProjectileVelocity` 4000.0)
      (set `self.FireRatePerSecond` 3.0)
      (set `self.Class` "/Game/RollingStarterPackV3/Blueprints/Hazards/Projectiles/Cannon_ProjectileMedium.Cannon_ProjectileMedium_C"))
    (:`NewEnumerator2`
      (`PrimitiveComponent.SetMaterial` _core 0 "/Game/RollingStarterPackV3/Materials/M_Inst/M_LightRed_Inst.M_LightRed_Inst")
      (set `self.ProjectileVelocity` 7000.0)
      (set `self.FireRatePerSecond` 5.0)
      (set `self.Class` "/Game/RollingStarterPackV3/Blueprints/Hazards/Projectiles/Cannon_ProjectileHard.Cannon_ProjectileHard_C"))))