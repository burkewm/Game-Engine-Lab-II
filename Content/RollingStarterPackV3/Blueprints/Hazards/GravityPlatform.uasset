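; GravityPlatform is a hazard platform that moves by an offset while a PhysicsBallBP keeps hitting it, then returns.
; A DoOnce-gated timeline lerps the mesh from its construction-time location toward that location plus EndLocation, at a play rate set by the inverse of PlatformMovementSpeed.
; Each hit restarts a one-second retriggerable delay, which resets the gate and reverses the timeline once hits stop.
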(event `self.StaticMesh.OnComponentHit`
  (params (HitComponent :type "PrimitiveComponent Object Reference") (OtherActor :type "Actor Object Reference") (OtherComp :type "PrimitiveComponent Object Reference") (NormalImpulse :type "Vector Structure") (Hit :type "HitResult Structure (by ref)"))
  (bind _starlocation (`self.StarLocation`))
  (cast `/Game/RollingStarterPackV3/Blueprints/PhysicsBallBP` OtherActor)
  (`|ExecutionSequence`
    (:`then_0`
      (`/Engine/EditorBlueprintResources/StandardMacros.DoOnce` false :!label _label
        (:`Completed`
          (`TimelineComponent.SetPlayRate` (`self.MovePlatform`) (/ 1.0 (`self.PlatformMovementSpeed`)))
          (bind (_direction _alpha) (`Timeline|MovePlatform` :!label _label_2)
            (:`Update`
              (`SceneComponent.K2_SetWorldLocation` (`self.StaticMesh`) (`KismetMathLibrary.VLerp` _starlocation (+ _starlocation (`self.EndLocation`)) _alpha) false false))))))
    (:`then_1`
      (`KismetSystemLibrary.RetriggerableDelay` 1.0)
      (`|ExecutionSequence`
        (:`then_0`
          (goto _label :!via `Reset`))
        (:`then_1`
          (goto _label_2 :!via `Reverse`))))))

(fn `UserConstructionScript`
  (set `self.StarLocation` (`SceneComponent.K2_GetComponentLocation` (`self.Root`))))