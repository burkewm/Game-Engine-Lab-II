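; Base power-up pickup for the rolling ball game, meant to be subclassed.
; Its mesh spins continuously on a looping timer.
; When a PhysicsBallBP overlaps its sphere, it copies its ability index, value and duration onto the ball and plays a pickup sound.
; It then disables overlaps until a respawn delay ends, leaving visibility changes to child Blueprints.
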(event `self.ReceiveBeginPlay`
  (`KismetSystemLibrary.K2_SetTimerDelegate` (delegate `Rotate`) 0.01 true))

(event `Rotate`
  (`SceneComponent.K2_AddRelativeRotation` (`self.PowerUpsMesh`) (struct :`Yaw` 1.0) false false))

(event `self.Sphere.OnComponentBeginOverlap`
  (params (OverlappedComponent :type "PrimitiveComponent Object Reference") (OtherActor :type "Actor Object Reference") (OtherComp :type "PrimitiveComponent Object Reference") (OtherBodyIndex :type Integer) (bFromSweep :type Boolean) (SweepResult :type "HitResult Structure (by ref)"))
  (bind _pickupsound (`self.PickUpSound`))
  ;[1 1 1] Set Values into physicsBall
  (bind _asphysics_ball_bp (cast `/Game/RollingStarterPackV3/Blueprints/PhysicsBallBP` OtherActor))
  (set `/Game/RollingStarterPackV3/Blueprints/PhysicsBallBP.AbilityIndexRef` (`self.Index`) _asphysics_ball_bp)
  (set `/Game/RollingStarterPackV3/Blueprints/PhysicsBallBP.PowerUpValue` (`self.Value`) _asphysics_ball_bp)
  (set `/Game/RollingStarterPackV3/Blueprints/PhysicsBallBP.PowerUpDuration` (`self.Duration`) _asphysics_ball_bp)
  ;[1 1 1] Make Overalp Respawn in N Second (visibility is set in child)
  (set `PrimitiveComponent.bGenerateOverlapEvents` false (`self.Sphere`))
  (`ActorComponent.SetActive` _pickupsound true false)
  (`AudioComponent.Play` _pickupsound 0.0)
  (`KismetSystemLibrary.Delay` (`self.RespawnDelay`))
  (set `PrimitiveComponent.bGenerateOverlapEvents` true (`self.Sphere`)))

(fn `UserConstructionScript`)