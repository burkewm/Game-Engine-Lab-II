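; PowerUp_Attach is a power-up Blueprint from the rolling-ball kit that gives its AbilityMesh custom gravity while the mesh simulates physics.
; Each Tick, it casts player pawn 0 to PhysicsBallBP and reads the up vector of that ball's GravityRoot.
; It scales that vector by TemporaryGravityForce and applies it as an acceleration, so the mesh follows the ball's gravity orientation independent of mass.
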(event `self.ReceiveTick`
  (params (DeltaSeconds :type "Float (single-precision)"))
  (if (`SceneComponent.IsSimulatingPhysics` (`self.AbilityMesh`) "None")
    (bind _asphysics_ball_bp (cast `/Game/RollingStarterPackV3/Blueprints/PhysicsBallBP` (`GameplayStatics.GetPlayerPawn` 0)))
    (`/Engine/EditorBlueprintResources/StandardMacros.IsValid` _asphysics_ball_bp
      (:`Is Valid`
        (`PrimitiveComponent.AddForce` (`self.AbilityMesh`) (* (`SceneComponent.GetUpVector` (`/Game/RollingStarterPackV3/Blueprints/PhysicsBallBP.GravityRoot` _asphysics_ball_bp)) (`self.TemporaryGravityForce`)) "None" true)))))

(fn `UserConstructionScript`)