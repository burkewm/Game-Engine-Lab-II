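; Gravity changer pickup that redirects a rolling PhysicsBallBP's gravity when the ball touches it.
; On overlap it plays a 2D sound and, if the ball's GravityRoot rotation differs from the collision sphere's, passes the sphere's rotation to GravityDirectionChanger.
; It then hides its particle, arrow and crystal visuals and disables overlaps until RespawnDelay elapses, when it reappears.
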(event `self.CollisionSphere.OnComponentBeginOverlap`
  (params (OverlappedComponent :type "PrimitiveComponent Object Reference") (OtherActor :type "Actor Object Reference") (OtherComp :type "PrimitiveComponent Object Reference") (OtherBodyIndex :type Integer) (bFromSweep :type Boolean) (SweepResult :type "HitResult Structure (by ref)"))
  (bind _returnvalue (`SceneComponent.K2_GetComponentRotation` (`self.CollisionSphere`)))
  (bind _asphysics_ball_bp (cast `/Game/RollingStarterPackV3/Blueprints/PhysicsBallBP` OtherActor))
  (`GameplayStatics.PlaySound2D` "/Game/RollingStarterPackV3/Audio/Cue/GravityNew_Cue.GravityNew_Cue" 1.0 1.0 0.0 null null)
  (if (!= (`SceneComponent.K2_GetComponentRotation` (`/Game/RollingStarterPackV3/Blueprints/PhysicsBallBP.GravityRoot` _asphysics_ball_bp)) _returnvalue)
    (`/Game/RollingStarterPackV3/Blueprints/PhysicsBallBP.GravityDirectionChanger` _asphysics_ball_bp _returnvalue))
  (`SceneComponent.SetVisibility` (`self.ParticleSystem`) false false)
  (`SceneComponent.SetVisibility` (`self.GravityDirectionMesh`) false false)
  (`SceneComponent.SetVisibility` (`self.CrystalMesh`) false false)
  (set `PrimitiveComponent.bGenerateOverlapEvents` false (`self.CollisionSphere`))
  (`KismetSystemLibrary.Delay` (`self.RespawnDelay`))
  (`SceneComponent.SetVisibility` (`self.ParticleSystem`) true false)
  (`SceneComponent.SetVisibility` (`self.GravityDirectionMesh`) true false)
  (`SceneComponent.SetVisibility` (`self.CrystalMesh`) true false)
  (set `PrimitiveComponent.bGenerateOverlapEvents` true (`self.CollisionSphere`)))

(fn `UserConstructionScript`)