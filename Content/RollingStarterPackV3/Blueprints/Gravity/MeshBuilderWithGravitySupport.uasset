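; Level-building actor that shows either a single mesh or a track of spline meshes, chosen by BuildTrack.
; The construction script syncs a per-point scale array to the spline, then creates one segment per point pair with roll and optional collision.
; Each segment takes both end scales from its starting point, so widths do not taper.
; Timed move and rotate timelines exist in the event graph, but nothing triggers them.
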(fn `Add Spline Mesh`
  (params (`Spline Index` :type Integer) (Mesh :type "StaticMesh Object Reference") (Material :type "MaterialInterface Object Reference"))
  (returns (LocalSplineMeshComponent1 :type "SplineMeshComponent Object Reference"))
  (locals (Local_End_Distance :type "Float (double-precision)") (Local_Start_Distance :type "Float (double-precision)") (Local_Mid_Distance :type "Float (double-precision)") (StartPos :type "Vector Structure" :default (0.0 0.0 0.0)) (StartTanget :type "Vector Structure" :default (0.0 0.0 0.0)) (EndPos :type "Vector Structure" :default (0.0 0.0 0.0)) (EndTanget :type "Vector Structure" :default (0.0 0.0 0.0)) (LocalSplineMeshComponent :type "SplineMeshComponent Object Reference") (LocalStaticMesh :type "StaticMesh Object Reference") (InSplineUPDir :type "Vector Structure") (Local_Rotation :type "Rotator Structure") (LocalStartRoll :type "Float (double-precision)") (LocalEndRoll :type "Float (double-precision)") (LocalStartWidth :type "Vector2D Structure") (LocalEndWidth :type "Vector2D Structure") (CurrentPoint :type Integer) (NextPoint :type Integer))
  (bind _localsplinemeshcomponent (`local.LocalSplineMeshComponent`))
  (bind _has_collision (`self.Has_Collision`))
  (bind _spline (`self.Spline`))
  (bind _local_end_distance (`local.Local_End_Distance`))
  (bind _local_mid_distance (`local.Local_Mid_Distance`))
  (bind _local_start_distance (`local.Local_Start_Distance`))
  (bind (_returnvalue _returnvalue2) (`self.GetPositionAndTanget` (`self.Spline`) _local_end_distance _local_end_distance))
  (bind (_returnvalue_2 _returnvalue2_2) (`self.GetPositionAndTanget` (`self.Spline`) (`local.Local_Start_Distance`) (`local.Local_End_Distance`)))
  (bind (_witdh _thickness) (break `/Game/RollingStarterPackV3/Blueprints/Gravity/SplineData` (`|GetArrayItem` (`self.SplinePointScale`) (`local.CurrentPoint`))))
  (bind (_witdh_2 _thickness_2) (break `/Game/RollingStarterPackV3/Blueprints/Gravity/SplineData` (`|GetArrayItem` (`self.SplinePointScale`) (`local.CurrentPoint`))))
  ;[1 1 1] Start and end spline point
  (bind _output_get (set `local.CurrentPoint` `Spline Index`))
  (set `local.NextPoint` (+ _output_get 1))
  (`|ExecutionSequence`
    (:`then_0`
      ;[1 1 1] Set start and end spline point distance
      (`|ExecutionSequence`
        (:`then_0`
          (set `local.Local_Start_Distance` (`SplineComponent.GetDistanceAlongSplineAtSplinePoint` (`self.Spline`) (`local.CurrentPoint`))))
        (:`then_1`
          (set `local.Local_End_Distance` (`SplineComponent.GetDistanceAlongSplineAtSplinePoint` (`self.Spline`) (`local.NextPoint`))))
        (:`then_2`
          (set `local.Local_Mid_Distance` (+ (/ (- (`local.Local_End_Distance`) _local_start_distance) 2.0) _local_start_distance)))
        (:`then_3`
          (set `local.LocalStaticMesh` Mesh))))
    (:`then_1`
      ;[1 1 1] Set spline data
      (set `local.StartPos` _returnvalue_2)
      (set `local.StartTanget` _returnvalue2_2)
      (set `local.EndPos` _returnvalue)
      (set `local.EndTanget` _returnvalue2)
      (set `local.InSplineUPDir` (`SplineComponent.GetUpVectorAtDistanceAlongSpline` _spline _local_mid_distance "Local"))
      (set `local.Local_Rotation` (`SplineComponent.GetRotationAtDistanceAlongSpline` _spline _local_mid_distance "Local"))
      (set `local.LocalStartRoll` (`KismetMathLibrary.MultiplyByPi` (/ (`self.GetRoll` (`self.Spline`) (`local.Local_Start_Distance`) (`local.Local_Rotation`)) 180.0)))
      (set `local.LocalEndRoll` (`KismetMathLibrary.MultiplyByPi` (/ (`self.GetRoll` (`self.Spline`) (`local.Local_End_Distance`) (`local.Local_Rotation`)) 180.0)))
      (set `local.LocalStartWidth` (`KismetMathLibrary.MakeVector2D` _witdh_2 _thickness_2))
      (set `local.LocalEndWidth` (`KismetMathLibrary.MakeVector2D` _witdh _thickness)))
    (:`then_2`
      ;[1 1 1] Add spline data and collison
      (bind _returnvalue_3 (`AddComponent|NODE_AddSplineMeshComponent-0`))
      (set `local.LocalSplineMeshComponent` _returnvalue_3)
      (`StaticMeshComponent.SetStaticMesh` (`local.LocalSplineMeshComponent`) (`local.LocalStaticMesh`))
      (`PrimitiveComponent.SetMaterial` _localsplinemeshcomponent 1 Material)
      (`SplineMeshComponent.SetSplineUpDir` _localsplinemeshcomponent (`local.InSplineUPDir`) true)
      (`SplineMeshComponent.SetStartAndEnd` (`local.LocalSplineMeshComponent`) (`local.StartPos`) (`local.StartTanget`) (`local.EndPos`) (`local.EndTanget`) true)
      (`SplineMeshComponent.SetStartRoll` (`local.LocalSplineMeshComponent`) (`local.LocalStartRoll`) true)
      (`SplineMeshComponent.SetEndRoll` (`local.LocalSplineMeshComponent`) (`local.LocalEndRoll`) true)
      (`SplineMeshComponent.SetStartScale` (`local.LocalSplineMeshComponent`) (`local.LocalStartWidth`) true)
      (`SplineMeshComponent.SetEndScale` (`local.LocalSplineMeshComponent`) (`local.LocalEndWidth`) true)
      (`PrimitiveComponent.SetCollisionEnabled` (`local.LocalSplineMeshComponent`) (select `bool` _has_collision :`false` "NoCollision" :`true` "QueryAndPhysics" :!type "ECollisionEnabled Enum"))
      (`PrimitiveComponent.SetCollisionResponseToAllChannels` (`local.LocalSplineMeshComponent`) (select `bool` _has_collision :`false` "ECR_Ignore" :`true` "ECR_Block" :!type "ECollisionResponse Enum")))
    (:`then_3`
      (return (`local.LocalSplineMeshComponent`)))))

(fn `UserConstructionScript`
  (bind _mesh (`self.Mesh`))
  (bind _mesh_2 (`self.Mesh`))
  (bind _splinepointscale (`self.SplinePointScale`))
  (bind _root (`self.Root`))
  (set `self.StartLocation` (`SceneComponent.K2_GetComponentLocation` _root))
  (set `self.StartRotation` (`SceneComponent.K2_GetComponentRotation` _root))
  (if (`self.BuildTrack`)
    (set `self.DoesRotate?` false)
    (set `self.DoesMove?` false)
    (`SceneComponent.SetVisibility` _mesh_2 false false)
    (`PrimitiveComponent.SetCollisionEnabled` _mesh_2 "NoCollision")
    (`|ExecutionSequence`
      (:`then_0`
        (set `self.NumberOfSplinePoints` (`SplineComponent.GetNumberOfSplinePoints` (`self.Spline`))))
      (:`then_1`
        ;[1 1 1] Add spline data scale
        (`/Engine/EditorBlueprintResources/StandardMacros.CompareInt` (`KismetArrayLibrary.Array_Length` (`self.SplinePointScale`)) (`self.NumberOfSplinePoints`) :!label _label
          (:`>`
            (`KismetArrayLibrary.Array_Remove` _splinepointscale (`KismetArrayLibrary.Array_LastIndex` _splinepointscale))
            (goto _label))
          (:`<`
            (`KismetArrayLibrary.Array_Add` (`self.SplinePointScale`))
            (goto _label))))
      (:`then_2`
        ;[1 1 1] Add spline point
        (for _index (range (+ (- (`self.NumberOfSplinePoints`) 2) 1))
          (bind _localsplinemeshcomponent1 (`self.Add Spline Mesh` _index (`self.SplineMesh`) (`self.Material`)))
          (bind _output_get (set `self.SplineMeshComponnent` _localsplinemeshcomponent1))
          (`PrimitiveComponent.SetMaterial` _output_get 0 (`self.SplineMaterial`)))))
    (else
      (`SceneComponent.SetVisibility` _mesh true false)
      (`PrimitiveComponent.SetCollisionEnabled` _mesh "QueryAndPhysics"))))